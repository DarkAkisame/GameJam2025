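; Rat enemy character that patrols via WalkForward and, when defeated, plays a delayed 2D Checkpoint sound.
; Tick runs forward wall and downward ledge traces, turning the rat when either finds an obstacle or drop.
; Capsule overlap damages the rat if the Cheeser player is dropping, otherwise damages the player and briefly halts walking.
; Defeat disables pawn collision response, plays a death montage, spawns healing Niagara, then destroys the actor.
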(event `self.ReceiveBeginPlay`
  (`parent.ReceiveBeginPlay`)
  (add `self.Defeted` (`|CreateDelegate` :!event `OnDefeted`)))

(event `OnDefeted`
  (bind (_returnvalue_location _returnvalue_rotation) (`KismetMathLibrary.BreakTransform` (`self.GetTransform`)))
  (`|ExecutionSequence`
    (:`then_0`
      (`KismetSystemLibrary.Delay` 1.0)
      (`GameplayStatics.PlaySound2D` "/Game/Cheeser/Audio/VO/Checkpoint.Checkpoint" 1.0 1.0 0.0 null null))
    (:`then_1`
      (`PrimitiveComponent.SetCollisionResponseToChannel` (`self.Rat_Capsile`) "ECC_Pawn" "ECR_Ignore")
      (bind _returnvalue (`self.PlayAnimMontage` "/Game/StylizedRatMount/Animations/A_Rat_Death_Montage.A_Rat_Death_Montage"))
      (`KismetSystemLibrary.Delay` _returnvalue)
      (`NiagaraFunctionLibrary.SpawnSystemAtLocation` "/Game/sA_PickupSet_1/Fx/NiagaraSystems/NS_Healing_1.NS_Healing_1" _returnvalue_location _returnvalue_rotation)
      (`self.K2_DestroyActor`))))

(event `self.Rat_Capsile.OnComponentBeginOverlap`
  (params (OverlappedComponent :type "PrimitiveComponent Object Reference") (OtherActor :type "Actor Object Reference") (OtherComp :type "PrimitiveComponent Object Reference") (OtherBodyIndex :type Integer) (bFromSweep :type Boolean) (SweepResult :type "HitResult Structure (by ref)"))
  (bind _asbp_cheeser_character (cast `/Game/Cheeser/Character/Player/BP_CheeserCharacter` OtherActor))
  (if (== (`Character.CapsuleComponent` _asbp_cheeser_character) OtherComp)
    (if (`/Game/Cheeser/Character/BP_CheeserPlayerController.IsDroping` (`/Game/Cheeser/Character/Player/BP_CheeserCharacter.Controller_Ref` _asbp_cheeser_character))
      (`GameplayStatics.ApplyDamage` self (`self.Over Lap Damage`) null _asbp_cheeser_character)
      (else
        (`GameplayStatics.ApplyDamage` _asbp_cheeser_character (`self.Over Lap Damage`) null self)
        (set `self.CanWalk` false)
        (`KismetSystemLibrary.Delay` 1.5)
        (set `self.CanWalk` true)))))

(event `WalkForward`
  (params (ScaleValue :type "Float (single-precision)" :default 1.0))
  (if (and (`self.CanWalk`) (not (`/Game/Cheeser/Blueprint/Componest/BPC_Stats.IsDefeated` (`self.BPC_Stats`))))
    (`self.AddMovementInput` (`self.GetActorForwardVector`) ScaleValue)))

(event `self.ReceiveTick`
  (params (DeltaSeconds :type "Float (single-precision)"))
  (`parent.ReceiveTick` DeltaSeconds)
  (if (not (`/Game/Cheeser/Blueprint/Componest/BPC_Stats.IsDefeated` (`self.BPC_Stats`)))
    (`self.EdjeDetect`)
    (`self.CheckifAnything isinFront`)))

(fn `CheckifAnything isinFront`
  (bind _capsulecomponent (`self.CapsuleComponent`))
  (bind _returnvalue (`SceneComponent.K2_GetComponentLocation` _capsulecomponent))
  (bind (_outhit _returnvalue_2) (`KismetSystemLibrary.LineTraceSingleForObjects` _returnvalue (+ _returnvalue (* (`SceneComponent.GetForwardVector` _capsulecomponent) (`self.Wall Check DIstnace`))) (`|MakeArray` "ObjectTypeQuery1" "ObjectTypeQuery2" :!type "EObjectTypeQuery Enum")))
  (if _returnvalue_2
    (`self.TurnCharacter`)))

(fn `EdjeDetect`
  (bind _capsulecomponent (`self.CapsuleComponent`))
  (bind _returnvalue (+ (`SceneComponent.K2_GetComponentLocation` _capsulecomponent) (* (`SceneComponent.GetForwardVector` _capsulecomponent) (`self.Wall Check DIstnace`))))
  (bind (_outhit _returnvalue_2) (`KismetSystemLibrary.LineTraceSingleForObjects` _returnvalue (+ _returnvalue (0.0 0.0 -100.0)) (`|MakeArray` "ObjectTypeQuery1" "ObjectTypeQuery2" :!type "EObjectTypeQuery Enum")))
  (if (not _returnvalue_2)
    (`self.TurnCharacter`)))

(fn `SetMaxWalkSpeed`
  (params (HasTarget :type Boolean))
  (set `CharacterMovementComponent.MaxWalkSpeed` (`KismetMathLibrary.SelectFloat` 400.0 100.0 HasTarget) (`self.CharacterMovement`)))

(fn `UserConstructionScript`
  (`parent.UserConstructionScript`))