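; Base enemy Blueprint for the Cheeser game that hurts the player's BP_CheeserCharacter on contact.
; When its capsule begins overlapping that character's capsule, it applies OverLapDamage with itself as the damage causer, ignoring the character's other components.
; A TurnCharacter function flips the enemy by combining its current rotation with a 180-degree offset, though nothing in this Blueprint calls it.
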(event `self.CapsuleComponent.OnComponentBeginOverlap`
  (params (OverlappedComponent :type "PrimitiveComponent Object Reference") (OtherActor :type "Actor Object Reference") (OtherComp :type "PrimitiveComponent Object Reference") (OtherBodyIndex :type Integer) (bFromSweep :type Boolean) (SweepResult :type "HitResult Structure (by ref)"))
  (bind _asbp_cheeser_character (cast `/Game/Cheeser/Character/Player/BP_CheeserCharacter` OtherActor))
  (if (== (`Character.CapsuleComponent` _asbp_cheeser_character) OtherComp)
    (`GameplayStatics.ApplyDamage` _asbp_cheeser_character (`self.Over Lap Damage`) null self)))

(fn `TurnCharacter`
  (`self.K2_SetActorRotation` (`KismetMathLibrary.ComposeRotators` (`self.K2_GetActorRotation`) (struct :`Yaw` 180.0))))

(fn `UserConstructionScript`
  (`parent.UserConstructionScript`))