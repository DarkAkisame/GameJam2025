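; Player character for a side-scrolling game, with X-axis movement, wall sliding, and a drop state owned by the player controller.
; While airborne, a forward trace flags wall jump and eases velocity toward zero, and gravity switches to the fall scale when descending in a drop.
; Enemy overlap damages the enemy during a drop, otherwise the player.
; Taking damage triggers invincibility, knockback and a timed stun flag.
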(event `self.ReceiveBeginPlay`
  (bind _asbp_cheeser_player_controller (cast `/Game/Cheeser/Character/BP_CheeserPlayerController` (`GameplayStatics.GetPlayerController` 0)))
  (set `self.Controller_Ref` _asbp_cheeser_player_controller)
  (set `self.Base_Gravity Scale` (`CharacterMovementComponent.GravityScale` (`self.CharacterMovement`))))

(event `EnhancedInput|/Game/Cheeser/Input/Action/IA_Move`
  (params (ActionValue :type "Float (double-precision)") (ElapsedSeconds :type "Float (double-precision)") (TriggeredSeconds :type "Float (double-precision)") (InputAction :type "InputAction Object Reference" :default "/Game/Cheeser/Input/Action/IA_Move.IA_Move"))
  (:`Triggered`
    (if (not (`/Game/Cheeser/Character/BP_CheeserPlayerController.IsDroping` (`self.Controller_Ref`)))
      (`self.AddMovementInput` (1.0 0.0 0.0) ActionValue)
      (`self.UpdateRotation` ActionValue))))

(event `UpdateRotationTrow`
  (params (Direction :type "Float (double-precision)"))
  (`self.UpdateRotation` Direction))

(event `self.ReceiveTick`
  (params (DeltaSeconds :type "Float (single-precision)"))
  (bind _charactermovement (`self.CharacterMovement`))
  (bind (_velocity_x _velocity_y _velocity_z) (`KismetMathLibrary.BreakVector` (`MovementComponent.Velocity` (`self.CharacterMovement`))))
  (if (`NavMovementInterface.IsFalling` (`self.CharacterMovement`))
    (`|ExecutionSequence`
      (:`then_0`
        (`self.HnadleWalllJump`))
      (:`then_1`
        (if (>= _velocity_z 0.0)
          (set `CharacterMovementComponent.GravityScale` (`self.Base_Gravity Scale`) _charactermovement)
          (elif (not (`/Game/Cheeser/Character/BP_CheeserPlayerController.IsDroping` (`self.Controller_Ref`)))
            (set `CharacterMovementComponent.GravityScale` (`self.Base_Gravity Scale`) _charactermovement)
            (else
              (set `CharacterMovementComponent.GravityScale` (`self.FallGRavityScale`) _charactermovement))))))
    (else
      (set `self.WallJump` false))))

(event `LaunchForm`
  (params (Impulse :type "Vector Structure"))
  (`CharacterMovementComponent.AddImpulse` (`self.CharacterMovement`) (`KismetMathLibrary.MakeVector` Impulse_X 0.0 Impulse_Z) true))

(event `self.ReceiveAnyDamage`
  (params (Damage :type "Float (single-precision)") (DamageType :type "DamageType Object Reference") (InstigatedBy :type "Controller Object Reference") (DamageCauser :type "Actor Object Reference"))
  (bind _returnvalue_x (`KismetMathLibrary.BreakVector` (`KismetMathLibrary.GetForwardVector` (`KismetMathLibrary.FindLookAtRotation` (`self.K2_GetActorLocation`) (`self.K2_GetActorLocation`)))))
  (`parent.ReceiveAnyDamage` Damage DamageType InstigatedBy DamageCauser)
  (`self.TiggerInvinciblity` (`self.CapsuleComponent`))
  (`self.LaunchCharacter` (`KismetMathLibrary.MakeVector` (* (`KismetMathLibrary.SelectFloat` -1.0 1.0 (> _returnvalue_x 0.0)) (`self.KnockBackPowerHorz`)) 0.0 (`self.KnockBackPowerVert`)) true true)
  (set `self.IsStuned` true)
  (`KismetSystemLibrary.RetriggerableDelay` (`self.StunedDuration`))
  (set `self.IsStuned` false))

(event `OverLapEnemey`
  (params (Enemy :type "/Game/Cheeser/Character/Enemyes/BP_EnemyBase Object Reference"))
  (if (`/Game/Cheeser/Character/BP_CheeserPlayerController.IsDroping` (`self.Controller_Ref`))
    (`GameplayStatics.ApplyDamage` Enemy (`self.Over Lap Damage`) null self)
    (else
      (`GameplayStatics.ApplyDamage` self (`self.Over Lap Damage`) null Enemy))))

(fn `HnadleWalllJump`
  (bind _capsulecomponent (`self.CapsuleComponent`))
  (bind _returnvalue (`SceneComponent.K2_GetComponentLocation` _capsulecomponent))
  (bind (_outhit _returnvalue_2) (`KismetSystemLibrary.LineTraceSingle` _returnvalue (+ _returnvalue (* (`SceneComponent.GetForwardVector` _capsulecomponent) (`self.WallCheckDIstnace`))) "TraceTypeQuery4"))
  (if _returnvalue_2
    (set `self.WallJump` true)
    (bind _charactermovement (`self.CharacterMovement`)
      (:`then`
        (set `MovementComponent.Velocity` (`KismetMathLibrary.VInterpTo_Constant` (`MovementComponent.Velocity` _charactermovement) (0.0 0.0 0.0) (`GameplayStatics.GetWorldDeltaSeconds`) (`self.WallFallSpeed`)) _charactermovement))
      (:`else`))
    (else
      (set `self.WallJump` false))))

(fn `Reset_Gravy_Scale`
  (set `CharacterMovementComponent.GravityScale` (`self.Base_Gravity Scale`) (`self.CharacterMovement`)))

(fn `SetGravityScale`
  (params (NewGravtyScale :type "Float (double-precision)"))
  (set `self.FallGRavityScale` NewGravtyScale))

(fn `UpdateRotation`
  (params (Direction :type "Float (double-precision)"))
  (`Controller.SetControlRotation` (`self.GetController`) (`KismetMathLibrary.SelectRotator` (struct) (struct :`Yaw` 180.0) (>= Direction 0.0))))

(fn `UserConstructionScript`)