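; Player controller that lets the player fling BP_CheeserCharacter by mouse-dragging its BP_FlingMouseGrab child actor.
; Each tick it traces under the cursor for hover, or moves the held grabber along the deprojected mouse ray.
; A float curve maps grabber-to-character distance to launch speed, visualized with debug shapes.
; Mouse release applies an X/Z-only velocity-change impulse toward the grabber, then resets the hovered grabber's position.
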(event `SetMouseGrabActor`
  (bind _flingermousegrab (`/Game/Cheeser/Character/BP_CheeserCharacter.FlingerMouseGrab` (`self.CheeserCharacter`)))
  (bind _asbp_fling_mouse_grab (cast `/Game/Cheeser/Fling/BP_FlingMouseGrab` (`ChildActorComponent.ChildActor` _flingermousegrab)))
  (set `self.MouseGrabActor` _asbp_fling_mouse_grab)
  (set `self.MouseGrabRelativePosition` (`SceneComponent.RelativeLocation` _flingermousegrab)))

(event `HoldGrabber`
  (bind (_worldlocation _worlddirection) (`self.DeprojectMousePositionToWorld`))
  (bind _lasthovered (`self.LastHovered`))
  (`/Engine/EditorBlueprintResources/StandardMacros.IsValid` (`self.MouseGrabActor`)
    (:`Is Valid`
      (`self.K2_SetActorLocation` (`self.MouseGrabActor`) (+ _worldlocation (* _worlddirection (`KismetMathLibrary.VSize` (- _worldlocation (`self.K2_GetActorLocation` (`self.CheeserCharacter`)))))) false false)
      (`/Engine/EditorBlueprintResources/StandardMacros.IsValid` _lasthovered
        (:`Is Valid`
          (`/Game/Cheeser/Fling/BP_FlingMouseGrab.SetHovered` _lasthovered true)
          (`self.CalculateVelocityPositionWithCurve`))))
    (:`Is Not Valid`
      (`self.SetMouseGrabActor`))))

(event `CalculateVelocityPositionWithCurve`
  (bind _velocitycurve (`self.VelocityCurve`))
  (if (and (`KismetSystemLibrary.IsValid` (`self.MouseGrabActor`)) (`KismetSystemLibrary.IsValid` (`self.CheeserCharacter`)))
    (`/Engine/EditorBlueprintResources/StandardMacros.IsValid` _velocitycurve
      (:`Is Valid`
        (set `self.LastVelocity` (`CurveFloat.GetFloatValue` _velocitycurve (`KismetMathLibrary.Vector_Distance` (`SceneComponent.K2_GetComponentLocation` (`/Game/Cheeser/Fling/BP_FlingMouseGrab.HoverSphere` (`self.MouseGrabActor`))) (`self.GetCharacterOffsetPosition`)))))
      (:`Is Not Valid`
        (`KismetSystemLibrary.PrintString` "YOU HAV ENO CURVE IN BP_CHEESERPLAYERCHARACTER!!")))
    (else
      (set `self.LastVelocity` 0.0))))

(event `Debug`
  (bind _returnvalue (- (`self.GetCharacterOffsetPosition`) (`SceneComponent.K2_GetComponentLocation` (`/Game/Cheeser/Fling/BP_FlingMouseGrab.HoverSphere` (`self.MouseGrabActor`)))))
  (if (and (`KismetSystemLibrary.IsValid` (`self.MouseGrabActor`)) (`KismetSystemLibrary.IsValid` (`self.VelocityCurve`)))
    ;[0.7147 0 1 0.5] Line from character to ball
    (`KismetSystemLibrary.DrawDebugLine` (`self.GetCharacterOffsetPosition`) (`SceneComponent.K2_GetComponentLocation` (`/Game/Cheeser/Fling/BP_FlingMouseGrab.HoverSphere` (`self.MouseGrabActor`))) (struct :`R` 1.0 :`G` 0.727112 :`A` 1.0) 0.066 3.0)
    ;[1 0.1537 0.1172 0.5] Second, smaller ball - opposite direction of the launch direction
    (`KismetSystemLibrary.DrawDebugSphere` (+ (`self.GetCharacterOffsetPosition`) (* (`KismetMathLibrary.Normal` _returnvalue) (* (`CurveFloat.GetFloatValue` (`self.VelocityCurve`) (`KismetMathLibrary.VSize` _returnvalue)) 0.2))) 12.0 12 (struct :`R` 1.0 :`G` 0.563558 :`A` 1.0) 0.066 3.3)))

(event `self.ReceiveBeginPlay`
  (set `self.bShowMouseCursor` true))

(event `self.ReceivePossess`
  (params (PossessedPawn :type "Pawn Object Reference"))
  (bind _asbp_cheeser_character (cast `/Game/Cheeser/Character/BP_CheeserCharacter` PossessedPawn))
  (set `self.CheeserCharacter` _asbp_cheeser_character))

(event `TraceForGrab`
  (bind (_start _end) (`self.GetMouseWorld`))
  (bind (_outhit _returnvalue) (`KismetSystemLibrary.LineTraceSingle` _start _end "TraceTypeQuery3" false (`|MakeArray` self (`self.K2_GetPawn`) :!type "Actor Object Reference")))
  (if _returnvalue
    (bind _asbp_fling_mouse_grab (cast `/Game/Cheeser/Fling/BP_FlingMouseGrab` (`.HitActor` (`GameplayStatics.BreakHitResult` _outhit))))
    (set `self.LastHovered` _asbp_fling_mouse_grab)
    (`/Game/Cheeser/Fling/BP_FlingMouseGrab.SetHovered` _asbp_fling_mouse_grab true)
    (`self.CalculateVelocityPositionWithCurve`)
    (elif (not (`self.HasCapturedFlingMesh`))
      (`/Engine/EditorBlueprintResources/StandardMacros.IsValid` (`self.LastHovered`)
        (:`Is Valid`
          (`/Game/Cheeser/Fling/BP_FlingMouseGrab.SetHovered` (`self.LastHovered`) false)
          (set `self.LastHovered` null)
          (set `self.HasCapturedFlingMesh` false))))))

(event `self.ReceiveUnPossess`
  (params (UnpossessedPawn :type "Pawn Object Reference"))
  (set `self.CheeserCharacter` null))

(event `self.ReceiveTick`
  (params (DeltaSeconds :type "Float (single-precision)"))
  (`self.Debug`)
  (if (`self.HasCapturedFlingMesh`)
    (`self.HoldGrabber`)
    (else
      (`self.TraceForGrab`))))

(event `LaunchCharacter`
  (`CharacterMovementComponent.AddImpulse` (`Character.CharacterMovement` (`self.CheeserCharacter`)) (`self.GetLaunchVelocity`) true)
  (set `self.LastVelocity` 0.0))

(event `InputAction|MouseClickEvent`
  (params (Key :type "Key Structure"))
  (:`Pressed`
    (`/Engine/EditorBlueprintResources/StandardMacros.IsValid` (`self.LastHovered`)
      (:`Is Valid`
        (set `self.HasCapturedFlingMesh` true))))
  (:`Released`
    (set `self.HasCapturedFlingMesh` false)
    (`self.LaunchCharacter`)
    (`self.ResetHovered`)))

(event `ResetHovered`
  (bind _lasthovered (`self.LastHovered`))
  (`/Engine/EditorBlueprintResources/StandardMacros.IsValid` _lasthovered
    (:`Is Valid`
      (`self.K2_SetActorLocation` _lasthovered (+ (`self.K2_GetActorLocation` (`self.CheeserCharacter`)) (`self.MouseGrabRelativePosition`)) false false))))

(fn `GetCharacterOffsetHeight`
  (returns (ReturnValue :type "Float (double-precision)"))
  (return (* (`CapsuleComponent.GetScaledCapsuleHalfHeight` (`Character.CapsuleComponent` (`self.CheeserCharacter`))) 0.75)))

(fn `GetCharacterOffsetPosition`
  (returns (ReturnValue :type "Vector Structure"))
  (return (+ (`self.K2_GetActorLocation` (`self.CheeserCharacter`)) (`KismetMathLibrary.MakeVector` 0.0 0.0 (`self.GetCharacterOffsetHeight`)))))

(fn `GetLaunchVelocity`
  (returns (ReturnValue :type "Vector Structure"))
  (bind (_returnvalue_x _returnvalue_y _returnvalue_z) (`KismetMathLibrary.BreakVector` (* (`KismetMathLibrary.Normal` (- (`SceneComponent.K2_GetComponentLocation` (`/Game/Cheeser/Fling/BP_FlingMouseGrab.HoverSphere` (`self.MouseGrabActor`))) (`self.GetCharacterOffsetPosition`))) (`self.LastVelocity`))))
  (return (`KismetMathLibrary.MakeVector` _returnvalue_x 0.0 _returnvalue_z)))

(fn `GetMouseWorld`
  (returns (Start :type "Vector Structure") (End :type "Vector Structure"))
  (bind (_worldlocation _worlddirection) (`self.DeprojectMousePositionToWorld`))
  (return _worldlocation (+ _worldlocation (* _worlddirection (`self.MouseGrabTraceDistance`)))))

(fn `UserConstructionScript`)