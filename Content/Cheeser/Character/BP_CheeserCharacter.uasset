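; Player character for Cheeser that moves along the X axis, with asymmetric jump gravity and wall sliding.
; Move input is blocked while the controller reports dropping, and control rotation flips to face the travel direction.
; While falling, gravity is heavier on descent, and a forward trace flags wall-jump state and eases velocity toward zero.
; Helpers apply X/Z launch impulses and set or restore gravity scale.
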(event `self.ReceiveBeginPlay`
  (bind _asbp_cheeser_player_controller (cast `/Game/Cheeser/Character/BP_CheeserPlayerController` (`GameplayStatics.GetPlayerController` 0)))
  (set `self.Controller_Ref` _asbp_cheeser_player_controller)
  (set `self.Base_Gravity Scale` (`CharacterMovementComponent.GravityScale` (`self.CharacterMovement`))))

(event `EnhancedInput|/Game/Cheeser/Input/Action/IA_Move`
  (params (ActionValue :type "Float (double-precision)") (ElapsedSeconds :type "Float (double-precision)") (TriggeredSeconds :type "Float (double-precision)") (InputAction :type "InputAction Object Reference" :default "/Game/Cheeser/Input/Action/IA_Move.IA_Move"))
  (:`Triggered`
    (if (not (`/Game/Cheeser/Character/BP_CheeserPlayerController.IsDroping` (`self.Controller_Ref`)))
      (`self.AddMovementInput` (1.0 0.0 0.0) ActionValue)
      (`self.UpdateRotation` ActionValue))))

(event `UpdateRotationTrow`
  (params (Direction :type "Float (double-precision)"))
  (`self.UpdateRotation` Direction))

(event `self.ReceiveTick`
  (params (DeltaSeconds :type "Float (single-precision)"))
  (bind _charactermovement (`self.CharacterMovement`))
  (bind (_velocity_x _velocity_y _velocity_z) (`KismetMathLibrary.BreakVector` (`MovementComponent.Velocity` (`self.CharacterMovement`))))
  (if (`NavMovementInterface.IsFalling` (`self.CharacterMovement`))
    (`|ExecutionSequence`
      (:`then_0`
        (`self.HnadleWalllJump`))
      (:`then_1`
        (if (>= _velocity_z 0.0)
          (set `CharacterMovementComponent.GravityScale` 1.0 _charactermovement)
          (else
            (set `CharacterMovementComponent.GravityScale` 2.0 _charactermovement)))))
    (else
      (set `self.WallJump` false))))

(event `LaunchForm`
  (params (Impulse :type "Vector Structure"))
  (`CharacterMovementComponent.AddImpulse` (`self.CharacterMovement`) (`KismetMathLibrary.MakeVector` Impulse_X 0.0 Impulse_Z) true))

(fn `HnadleWalllJump`
  (bind _capsulecomponent (`self.CapsuleComponent`))
  (bind _returnvalue (`SceneComponent.K2_GetComponentLocation` _capsulecomponent))
  (bind (_outhit _returnvalue_2) (`KismetSystemLibrary.LineTraceSingle` :`Start` _returnvalue :`End` (+ _returnvalue (* (`SceneComponent.GetForwardVector` _capsulecomponent) (`self.WallCheckDIstnace`))) :`TraceChannel` "TraceTypeQuery4" :`DrawDebugType` "ForDuration"))
  (if _returnvalue_2
    (set `self.WallJump` true)
    (bind _charactermovement (`self.CharacterMovement`)
      (:`then`
        (set `MovementComponent.Velocity` (`KismetMathLibrary.VInterpTo_Constant` (`MovementComponent.Velocity` _charactermovement) (0.0 0.0 0.0) (`GameplayStatics.GetWorldDeltaSeconds`) (`self.WallFallSpeed`)) _charactermovement))
      (:`else`))
    (else
      (set `self.WallJump` false))))

(fn `Reset_Gravy_Scale`
  (set `CharacterMovementComponent.GravityScale` (`self.Base_Gravity Scale`) (`self.CharacterMovement`)))

(fn `SetGravityScale`
  (params (NewGravtyScale :type "Float (double-precision)"))
  (set `CharacterMovementComponent.GravityScale` NewGravtyScale (`self.CharacterMovement`)))

(fn `UpdateRotation`
  (params (Direction :type "Float (double-precision)"))
  (`Controller.SetControlRotation` (`self.GetController`) (`KismetMathLibrary.SelectRotator` (struct) (struct :`Yaw` 180.0) (>= Direction 0.0))))

(fn `UserConstructionScript`)