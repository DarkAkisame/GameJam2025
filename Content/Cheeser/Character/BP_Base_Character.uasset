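; Base character Blueprint providing shared damage, defeat, invincibility and facing logic.
; Incoming damage goes to the BPCStats component until defeated, then the defeat call fires.
; Triggered invincibility makes a given capsule ignore Pawns and flickers the mesh on a looping timer, restoring overlap and visibility after a retriggerable delay.
; UpdateRotation flips control rotation 180 degrees according to the sign of movement direction.
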(event `self.ReceiveAnyDamage`
  (params (Damage :type "Float (single-precision)") (DamageType :type "DamageType Object Reference") (InstigatedBy :type "Controller Object Reference") (DamageCauser :type "Actor Object Reference"))
  (bind _bpc_stats (`self.BPC_Stats`))
  (if (not (`/Game/Cheeser/Blueprint/Componest/BPC_Stats.IsDefeated` (`self.BPC_Stats`)))
    (`/Game/Cheeser/Blueprint/Componest/BPC_Stats.ReceviveDamage` _bpc_stats Damage)
    (if (`/Game/Cheeser/Blueprint/Componest/BPC_Stats.IsDefeated` _bpc_stats)
      (`self.Defeted`))))

(event `TiggerInvinciblity`
  (params (DamgeCapsuleComp :type "CapsuleComponent Object Reference"))
  (`/Engine/EditorBlueprintResources/StandardMacros.IsValid` DamgeCapsuleComp
    (:`Is Valid`
      (`PrimitiveComponent.SetCollisionResponseToChannel` DamgeCapsuleComp "ECC_Pawn" "ECR_Ignore")
      (bind _returnvalue (`KismetSystemLibrary.K2_SetTimerDelegate` (`|CreateDelegate` :!event `ToggleMeshVisbility`) (`self.MeshFlickerInterval`) true))
      (set `self.VisbilityHandel` _returnvalue)
      (`KismetSystemLibrary.RetriggerableDelay` (`self.InvinbilityDutation`))
      (`KismetSystemLibrary.K2_ClearAndInvalidateTimerHandle` (`self.VisbilityHandel`))
      (`PrimitiveComponent.SetCollisionResponseToChannel` DamgeCapsuleComp "ECC_Pawn" "ECR_Overlap")
      (`SceneComponent.SetVisibility` (`self.Mesh`) true true))))

(fn `ToggleMeshVisbility`
  (bind _mesh (`self.Mesh`))
  (`SceneComponent.SetVisibility` _mesh (not (`SceneComponent.bVisible` _mesh)) false))

(fn `UpdateRotation`
  (params (Direction :type "Float (double-precision)"))
  (`Controller.SetControlRotation` (`self.GetController`) (`KismetMathLibrary.SelectRotator` (struct) (struct :`Yaw` 180.0) (>= Direction 0.0))))

(fn `UserConstructionScript`)