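; Game mode for Cheeser that owns the HUD, tracks player lives and handles respawning.
; BeginPlay creates WBP_HUD, caches the level's PlayerStart and pushes the initial life count to the lives widget.
; RespawnPlayer decrements lives without a zero check and updates the HUD.
; It then spawns and possesses a new default pawn at the active checkpoint, falling back to PlayerStart when none is valid.
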(event `self.ReceiveBeginPlay`
  (`|ExecutionSequence`
    (:`then_0`
      (bind _returnvalue (`|CreateWidget` "/Game/Cheeser/Blueprint/Widgets/WBP_HUD.WBP_HUD_C"))
      (bind _output_get (set `self.HUD_Ref` _returnvalue))
      (`UserWidget.AddToViewport` _output_get 0))
    (:`then_1`
      (bind _returnvalue_2 (`GameplayStatics.GetActorOfClass` "/Script/Engine.PlayerStart"))
      (set `self.PlayerStart` _returnvalue_2)
      (`/Game/Cheeser/Blueprint/Widgets/WBP_Lives.UpdateLives` (`/Game/Cheeser/Blueprint/Widgets/WBP_HUD.WBP_Lives` (`self.HUD_Ref`)) (`self.Lives`)))))

(event `self.ReceiveTick`
  (params (DeltaSeconds :type "Float (single-precision)")))

(fn `RespawnPlayer`
  (bind (_returnvalue_location _returnvalue_rotation) (`KismetMathLibrary.BreakTransform` (`self.GetTransform` (`self.PlayerStart`))))
  (bind (_returnvalue_location_2 _returnvalue_rotation_2) (`KismetMathLibrary.BreakTransform` (`SceneComponent.K2_GetComponentToWorld` (`/Game/Cheeser/Blueprint/BP_CheckPoint.Scene` (`self.ActiveCheckPoint`)))))
  (`/Engine/EditorBlueprintResources/StandardMacros.DecrementInt` (`self.Lives`)
    (:`  `
      (`/Game/Cheeser/Blueprint/Widgets/WBP_Lives.UpdateLives` (`/Game/Cheeser/Blueprint/Widgets/WBP_HUD.WBP_Lives` (`self.HUD_Ref`)) (`self.Lives`))
      (`/Engine/EditorBlueprintResources/StandardMacros.IsValid` (`self.ActiveCheckPoint`)
        (:`Is Valid`
          (bind _returnvalue (`|SpawnActorFromClass` (`self.DefaultPawnClass`) (`KismetMathLibrary.MakeTransform` _returnvalue_location_2 _returnvalue_rotation_2) "Undefined" "MultiplyWithRoot" null null))
          (`Controller.Possess` (`GameplayStatics.GetPlayerController` 0) _returnvalue))
        (:`Is Not Valid`
          (bind _returnvalue_2 (`|SpawnActorFromClass` (`self.DefaultPawnClass`) (`KismetMathLibrary.MakeTransform` _returnvalue_location _returnvalue_rotation) "Undefined" "MultiplyWithRoot" null null))
          (`Controller.Possess` (`GameplayStatics.GetPlayerController` 0) _returnvalue_2))))))

(fn `UserConstructionScript`)