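; BP_SmashBox is a breakable box that the Cheeser character smashes by dropping onto it.
; When its Box component is overlapped by BP_CheeserCharacter while that character's controller reports IsDroping, the mesh starts ignoring Pawn collision.
; It then plays a smash sound and explosion effect, spawns BP_Heath at SpawnLocation on two chained coin flips (25% chance), and destroys itself.
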(event `self.Box.OnComponentBeginOverlap`
  (params (OverlappedComponent :type "PrimitiveComponent Object Reference") (OtherActor :type "Actor Object Reference") (OtherComp :type "PrimitiveComponent Object Reference") (OtherBodyIndex :type Integer) (bFromSweep :type Boolean) (SweepResult :type "HitResult Structure (by ref)"))
  (bind (_returnvalue_location _returnvalue_rotation) (`KismetMathLibrary.BreakTransform` (`self.GetTransform`)))
  (bind (_returnvalue_location_2 _returnvalue_rotation_2) (`KismetMathLibrary.BreakTransform` (`SceneComponent.K2_GetComponentToWorld` (`self.SpawnLocation`))))
  (bind _asbp_cheeser_character (cast `/Game/Cheeser/Character/Player/BP_CheeserCharacter` OtherActor))
  (if (`/Game/Cheeser/Character/BP_CheeserPlayerController.IsDroping` (`/Game/Cheeser/Character/Player/BP_CheeserCharacter.Controller_Ref` _asbp_cheeser_character))
    (`PrimitiveComponent.SetCollisionResponseToChannel` (`self.StaticMesh`) "ECC_Pawn" "ECR_Ignore")
    (`GameplayStatics.PlaySound2D` "/Game/Cheeser/Audio/FX/Smash.Smash" 1.0 1.0 0.0 null null)
    (`GameplayStatics.SpawnEmitterAtLocation` "/Game/StarterContent/Particles/P_Explosion.P_Explosion" _returnvalue_location _returnvalue_rotation)
    (if (`KismetMathLibrary.RandomBool`)
      (if (`KismetMathLibrary.RandomBool`)
        (`|SpawnActorFromClass` "/Game/Cheeser/Blueprint/BP_Heath.BP_Heath_C" (`KismetMathLibrary.MakeTransform` _returnvalue_location_2 _returnvalue_rotation_2) "Undefined" "MultiplyWithRoot" null null)))
    (`self.K2_DestroyActor`)))

(fn `UserConstructionScript`)