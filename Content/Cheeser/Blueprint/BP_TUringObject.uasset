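; BP_TUringObject is an actor that carries another actor along by position, without engine attachment.
; AttachLocation stores the target and moves the Scene component to the target's location, converted into this actor's local space.
; While attached, Tick sets the target's world location to the Scene component's, so it follows this actor's transform but keeps its own rotation.
; UnattachActor clears the reference and stops the following.
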(event `self.ReceiveTick`
  (params (DeltaSeconds :type "Float (single-precision)"))
  (if (`self.ActorIsAttached`)
    (bind _attach_actor (`self.Attach Actor`)
      (:`then`
        (`self.K2_SetActorLocation` _attach_actor (`SceneComponent.K2_GetComponentLocation` (`self.Scene`)) false false))
      (:`else`))))

(event `/Game/Cheeser/Blueprint/Interfaces/BPI_AttachTo.AttachLocation`
  (params (AttachActor :type "Actor Object Reference"))
  (bind _output_get (set `self.Attach Actor` AttachActor))
  (set `self.ActorIsAttached` true)
  (`SceneComponent.K2_SetRelativeLocation` (`self.Scene`) (`KismetMathLibrary.InverseTransformLocation` (`self.GetTransform`) (`self.K2_GetActorLocation` _output_get)) false false))

(event `/Game/Cheeser/Blueprint/Interfaces/BPI_AttachTo.UnattachActor`
  (set `self.ActorIsAttached` false)
  (set `self.Attach Actor` null))

(fn `UserConstructionScript`)