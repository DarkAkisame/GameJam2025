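; BP_TutTimeSlow is a tutorial trigger, named for time slow, that plays a voice-over when the Cheeser character enters its box.
; The overlap also enables input so IA_Skip can stop the audio, with HasPlayed and a DoOnce guarding against replays.
; Audio finish and skip share one cleanup path that disables the trigger, clears the mesh, calls CallKillValume, destroys the Block component and disables input.
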(event `self.Box_Trigger.OnComponentBeginOverlap`
  (params (OverlappedComponent :type "PrimitiveComponent Object Reference") (OtherActor :type "Actor Object Reference") (OtherComp :type "PrimitiveComponent Object Reference") (OtherBodyIndex :type Integer) (bFromSweep :type Boolean) (SweepResult :type "HitResult Structure (by ref)"))
  (cast `/Game/Cheeser/Character/Player/BP_CheeserCharacter` OtherActor)
  (if (not (`self.HasPlayed`))
    (`/Engine/EditorBlueprintResources/StandardMacros.DoOnce` (`self.HasPlayed`)
      (:`Completed`
        (`AudioComponent.Play` (`self.VO_Audio`) 0.0)
        (`self.EnableInput` (`GameplayStatics.GetPlayerController` 0))))))

(event `self.VO_Audio.OnAudioFinished`
  (`PrimitiveComponent.SetCollisionEnabled` (`self.Box_Trigger`) "NoCollision" :!label _label)
  (`StaticMeshComponent.SetStaticMesh` (`self.StaticMesh`) null)
  (set `self.HasPlayed` true)
  (`self.KillValume`)
  (`ActorComponent.K2_DestroyComponent` (`self.block`))
  (`self.DisableInput` (`GameplayStatics.GetPlayerController` 0)))

(event `EnhancedInput|/Game/Cheeser/Input/Action/IA_Skip`
  (params (ActionValue :type Boolean) (ElapsedSeconds :type "Float (double-precision)") (TriggeredSeconds :type "Float (double-precision)") (InputAction :type "InputAction Object Reference" :default "/Game/Cheeser/Input/Action/IA_Skip.IA_Skip"))
  (:`Triggered`
    (`AudioComponent.Stop` (`self.VO_Audio`))
    (goto _label)))

(fn `UserConstructionScript`)