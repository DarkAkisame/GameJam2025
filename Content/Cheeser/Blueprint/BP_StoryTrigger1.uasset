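; BP_StoryTrigger1 is a one-shot story trigger that plays a voice-over when the player character, BP_CheeserCharacter, enters its box.
; On overlap, it pauses the game and starts the VO audio, provided it has not already played.
; When the audio finishes, it unpauses the game, disables the box's collision and sets HasPlayed so the line does not repeat.
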(event `self.Box_Trigger.OnComponentBeginOverlap`
  (params (OverlappedComponent :type "PrimitiveComponent Object Reference") (OtherActor :type "Actor Object Reference") (OtherComp :type "PrimitiveComponent Object Reference") (OtherBodyIndex :type Integer) (bFromSweep :type Boolean) (SweepResult :type "HitResult Structure (by ref)"))
  (cast `/Game/Cheeser/Character/Player/BP_CheeserCharacter` OtherActor)
  (if (not (`self.HasPlayed`))
    (`GameplayStatics.SetGamePaused` true)
    (`AudioComponent.Play` (`self.VO_Audio`) 0.0)))

(event `self.VO_Audio.OnAudioFinished`
  (`GameplayStatics.SetGamePaused` false)
  (`PrimitiveComponent.SetCollisionEnabled` (`self.Box_Trigger`) "NoCollision")
  (set `self.HasPlayed` true))

(fn `UserConstructionScript`)