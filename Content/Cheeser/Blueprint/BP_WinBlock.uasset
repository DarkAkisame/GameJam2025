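; BP_WinBlock is a level gate that blocks the player until enough curds are collected.
; On BeginPlay it caches the Cheeser player controller and binds CanWInLevel to the controller's curd-check event.
; When that event fires with the count at or above CurdesToWin, the block drops its collision and its static mesh is set.
; If the player overlaps the block while short of curds, a YouNeedMore cue plays.
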(event `self.ReceiveBeginPlay`
  (bind _asbp_cheeser_player_controller (cast `/Game/Cheeser/Character/BP_CheeserPlayerController` (`GameplayStatics.GetPlayerController` 0)))
  (set `self.playerControl_ref` _asbp_cheeser_player_controller)
  (add `/Game/Cheeser/Character/BP_CheeserPlayerController.CheckIfYouHaveCurdsNeeded` _asbp_cheeser_player_controller (delegate `CanWInLevel`)))

(event `CanWInLevel`
  (if (>= (`/Game/Cheeser/Character/BP_CheeserPlayerController.NumOfCurdes` (`self.playerControl_ref`)) (`self.CurdesToWin`))
    (`PrimitiveComponent.SetCollisionEnabled` (`self.block`) "NoCollision")
    (`StaticMeshComponent.SetStaticMesh` (`self.StaticMesh`) null)))

(event `self.block.OnComponentBeginOverlap`
  (params (OverlappedComponent :type "PrimitiveComponent Object Reference") (OtherActor :type "Actor Object Reference") (OtherComp :type "PrimitiveComponent Object Reference") (OtherBodyIndex :type Integer) (bFromSweep :type Boolean) (SweepResult :type "HitResult Structure (by ref)"))
  (if (and (not (>= (`/Game/Cheeser/Character/BP_CheeserPlayerController.NumOfCurdes` (`self.playerControl_ref`)) (`self.CurdesToWin`))) (== OtherActor (`GameplayStatics.GetPlayerCharacter` 0)))
    (`AudioComponent.Play` (`self.YouNeedMore`) 0.0)))

(fn `UserConstructionScript`)