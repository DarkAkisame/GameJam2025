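; BP_Cannon is an actor that loads an overlapping Cheeser character and launches it through the air.
; The seat trigger stores the Occupant, disables its input, collision and movement, hides it and snaps it to the Muzzle.
; IA_Fire plays sound and exhaust effects, then restores and launches any occupant along the Muzzle's forward vector.
; A short timer re-enables player input and clears the seat.
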(event `self.SeatTrigger.OnComponentBeginOverlap`
  (params (OverlappedComponent :type "PrimitiveComponent Object Reference") (OtherActor :type "Actor Object Reference") (OtherComp :type "PrimitiveComponent Object Reference") (OtherBodyIndex :type Integer) (bFromSweep :type Boolean) (SweepResult :type "HitResult Structure (by ref)"))
  (bind _muzzle (`self.Muzzle`))
  (bind _occupant (`self.Occupant`))
  (bind _returnvalue (`Pawn.GetController` (`self.Occupant`)))
  (bind _asbp_cheeser_character (cast `/Game/Cheeser/Character/Player/BP_CheeserCharacter` OtherActor))
  (if (not (`KismetSystemLibrary.IsValid` (`self.Occupant`)))
    (set `self.Occupant` _asbp_cheeser_character)
    (bind _asbp_cheeser_player_controller (cast `/Game/Cheeser/Character/BP_CheeserPlayerController` _returnvalue))
    (`self.DisableInput` _returnvalue _asbp_cheeser_player_controller)
    (`PrimitiveComponent.SetCollisionEnabled` (`Character.CapsuleComponent` _occupant) "NoCollision")
    (`CharacterMovementComponent.SetMovementMode` (`Character.CharacterMovement` _occupant) "MOVE_None" 0)
    (`self.SetActorHiddenInGame` (`self.Occupant`) true)
    (`self.K2_AttachToComponent` (`self.Occupant`) _muzzle "None" "SnapToTarget" "SnapToTarget" "SnapToTarget" true)
    (`self.K2_SetActorTransform` (`self.Occupant`) (`SceneComponent.K2_GetComponentToWorld` _muzzle) false true)))

(event `EnhancedInput|/Game/Cheeser/Input/Action/IA_Fire`
  (params (ActionValue :type Boolean) (ElapsedSeconds :type "Float (double-precision)") (TriggeredSeconds :type "Float (double-precision)") (InputAction :type "InputAction Object Reference" :default "/Game/Cheeser/Input/Action/IA_Fire.IA_Fire"))
  (bind _occupant (`self.Occupant`))
  (:`Triggered`
    (`GameplayStatics.PlaySound2D` "/Game/Cheeser/Audio/FX/cannon_FX.cannon_FX" 1.0 1.0 0.0 null null)
    (`|ExecutionSequence`
      (:`then_0`
        (`NiagaraFunctionLibrary.SpawnSystemAtLocation` "/Game/RocketThrusterExhaustFX/FX/NS_RocketExhaust_Violet.NS_RocketExhaust_Violet" (`self.K2_GetActorLocation` (stale `self.SeatTrigger.OnComponentBeginOverlap` _asbp_cheeser_character))))
      (:`then_1`
        (`self.Occupant`
          (:`then`
            (`self.SetActorHiddenInGame` (`self.Occupant`) false)
            (`self.K2_DetachFromActor` (`self.Occupant`) "KeepWorld" "KeepWorld" "KeepWorld")
            (`PrimitiveComponent.SetCollisionEnabled` (`Character.CapsuleComponent` _occupant) "QueryAndPhysics")
            (`CharacterMovementComponent.SetMovementMode` (`Character.CharacterMovement` _occupant) "MOVE_Falling" 0)
            (`/Game/Cheeser/Character/Player/BP_CheeserCharacter.LaunchForm ` (`self.Occupant`) (* (`KismetMathLibrary.GetForwardVector` (`SceneComponent.K2_GetComponentRotation` (`self.Muzzle`))) (`self.LaunchSpeed`)))
            (`KismetSystemLibrary.K2_SetTimerDelegate` (delegate `EnablePlayerInput`) 0.1))
          (:`else`
            (`KismetSystemLibrary.PrintString` "No Occupent")))))))

(event `EnablePlayerInput`
  (bind _returnvalue (`Pawn.GetController` (`self.Occupant`)))
  (bind _asbp_cheeser_player_controller (cast `/Game/Cheeser/Character/BP_CheeserPlayerController` _returnvalue))
  (`self.EnableInput` _returnvalue _asbp_cheeser_player_controller)
  (set `self.Occupant` null))

(fn `UserConstructionScript`)