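; AI controller for the rat enemy, which keeps its possessed rat walking forward on every tick.
; AI perception updates store the first player character as the attack target and toggle the rat's max walk speed.
; An update for any other actor clears the target and reverts the speed flag; whether the stimulus was sensed or lost is not checked.
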(event `self.ReceivePossess`
  (params (PossessedPawn :type "Pawn Object Reference"))
  (bind _asbp_enemy_rat (cast `/Game/Cheeser/Character/Enemyes/BP_Enemy_Rat` PossessedPawn))
  (set `self.OwningRat` _asbp_enemy_rat))

(event `self.ReceiveTick`
  (params (DeltaSeconds :type "Float (single-precision)"))
  (bind _owningrat (`self.OwningRat`)
    (:`then`
      (`/Game/Cheeser/Character/Enemyes/BP_Enemy_Rat.WalkForward` _owningrat 1.0))
    (:`else`)))

(event `self.AIPerception.OnTargetPerceptionUpdated`
  (params (Actor :type "Actor Object Reference") (Stimulus :type "AIStimulus Structure"))
  (bind _owningrat (`self.OwningRat`))
  (if (== Actor (`GameplayStatics.GetPlayerCharacter` 0))
    (set `self.AtttackTarget` Actor)
    (`/Engine/EditorBlueprintResources/StandardMacros.IsValid` _owningrat
      (:`Is Valid`
        (`/Game/Cheeser/Character/Enemyes/BP_Enemy_Rat.SetMaxWalkSpeed` _owningrat true)))
    (else
      (set `self.AtttackTarget` null)
      (`/Engine/EditorBlueprintResources/StandardMacros.IsValid` _owningrat
        (:`Is Valid`
          (`/Game/Cheeser/Character/Enemyes/BP_Enemy_Rat.SetMaxWalkSpeed` _owningrat false))))))

(fn `UserConstructionScript`
  (`parent.UserConstructionScript`))