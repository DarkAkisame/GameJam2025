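; BP_CheckPoint is a checkpoint actor that becomes the active checkpoint when the player character touches it.
; It caches the game mode on BeginPlay and registers itself as ActiveCheckPoint there when a BP_CheeserCharacter overlaps its box.
; The previously active checkpoint's mesh reverts to the default material, while the new one switches to a highlight material, so only one shows as active.
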(event `self.ReceiveBeginPlay`
  (bind _asbp_cheeser_game_mode (cast `/Game/Cheeser/BP_CheeserGameMode` (`GameplayStatics.GetGameMode`)))
  (set `self.GameMode_REf` _asbp_cheeser_game_mode))

(event `self.Box.OnComponentBeginOverlap`
  (params (OverlappedComponent :type "PrimitiveComponent Object Reference") (OtherActor :type "Actor Object Reference") (OtherComp :type "PrimitiveComponent Object Reference") (OtherBodyIndex :type Integer) (bFromSweep :type Boolean) (SweepResult :type "HitResult Structure (by ref)"))
  (cast `/Game/Cheeser/Character/Player/BP_CheeserCharacter` OtherActor)
  (`/Engine/EditorBlueprintResources/StandardMacros.IsValid` (`/Game/Cheeser/BP_CheeserGameMode.ActiveCheckPoint` (`self.GameMode_REf`))
    (:`Is Valid`
      (if (not (== (`/Game/Cheeser/BP_CheeserGameMode.ActiveCheckPoint` (`self.GameMode_REf`)) self))
        (`PrimitiveComponent.SetMaterial` (`/Game/Cheeser/Blueprint/BP_CheckPoint.StaticMesh` (`/Game/Cheeser/BP_CheeserGameMode.ActiveCheckPoint` (`self.GameMode_REf`))) 0 "/Game/CharacterBodyFX/Materials/MM_CheckPoint.MM_CheckPoint")
        (set `/Game/Cheeser/BP_CheeserGameMode.ActiveCheckPoint` self (`self.GameMode_REf`))
        (`PrimitiveComponent.SetMaterial` (`self.StaticMesh`) 0 "/Game/CharacterBodyFX/Materials/MI_CHeckPointColor2.MI_CHeckPointColor2")))
    (:`Is Not Valid`
      (set `/Game/Cheeser/BP_CheeserGameMode.ActiveCheckPoint` self (`self.GameMode_REf`))
      (`PrimitiveComponent.SetMaterial` (`self.StaticMesh`) 0 "/Game/CharacterBodyFX/Materials/MI_CHeckPointColor2.MI_CHeckPointColor2"))))

(fn `UserConstructionScript`)